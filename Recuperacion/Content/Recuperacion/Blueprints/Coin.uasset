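; Coin pickup actor that adds to the player's coin count on the HUD when its sphere is touched.
; Any overlap on the Sphere component calls AddCoin and then destroys the actor, without checking what overlapped it.
; AddCoin casts player 0 to ThirdPersonCharacter, plays the HUD's coin animation and increments the Coins value stored on that HUD.
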(event OnComponentBeginOverlap(Sphere)
  (params (OverlappedComponent :type Primitive%20Component%20Object%20Reference) (OtherActor :type Actor%20Object%20Reference) (OtherComp :type Primitive%20Component%20Object%20Reference) (OtherBodyIndex :type Integer) (bFromSweep :type Boolean) (SweepResult :type Hit%20Result%20Structure%20%28by%20ref%29))
  (CallFunction|AddCoin)
  (Actor|DestroyActor))

(event EventBeginPlay)

(event Collision|EventActorBeginOverlap
  (params (OtherActor :type Actor%20Object%20Reference)))

(event EventTick
  (params (DeltaSeconds :type Float%20%28single-precision%29)))

(fn ConstructionScript)

(fn AddCoin
  (bind _asthird_person_character (Utilities|Casting|CastToThirdPersonCharacter (Game|GetPlayerCharacter 0)))
  (UserInterface|Animation|PlayAnimation (Variables|/Game/ThirdPersonBP/Blueprints/ThirdPersonCharacter.ThirdPersonCharacter_C|GetHud _asthird_person_character) (Variables|/Game/Recuperacion/Blueprints/HUD.HUD_C|GetCoinsAnim (Variables|/Game/ThirdPersonBP/Blueprints/ThirdPersonCharacter.ThirdPersonCharacter_C|GetHud _asthird_person_character)) 0.0 1 "Forward" 1.0 false)
  (Variables|/Game/Recuperacion/Blueprints/HUD.HUD_C|SetCoins (Variables|/Game/ThirdPersonBP/Blueprints/ThirdPersonCharacter.ThirdPersonCharacter_C|GetHud _asthird_person_character) (+ (Variables|/Game/Recuperacion/Blueprints/HUD.HUD_C|GetCoins (Variables|/Game/ThirdPersonBP/Blueprints/ThirdPersonCharacter.ThirdPersonCharacter_C|GetHud _asthird_person_character)) 1)))